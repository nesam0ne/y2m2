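; BP_Tile is a single grid cell that tracks whether a block occupies it.
; Initialize attaches the tile to its owner and offsets it by Column and Row, using the Plane's bounds as spacing.
; Overlap with BP_block or BP_longblock sets IsTaken, and any end overlap clears it.
; BeginPlay enables mouse clicks, but the click handler only checks IsWin and IsTaken around a delay, with no resulting action.
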(event Custom|OnClicked_Event
  (params (TouchedActor :type Actor%20Object%20Reference) (ButtonPressed :type Key%20Structure :default "None"))
  (if (Variables|Default|GetIsWin)
    (Utilities|FlowControl|Delay 0.3)
    (if (not (Variables|Default|GetIsTaken))
      _)))

(event EventBeginPlay
  (Variables|/Script/Engine.PlayerController|SetbEnableClickEvents (Game|GetPlayerController 0) true)
  (EventDispatchers|BindEventtoOnClicked (delegate Custom|OnClicked_Event)))

(event Collision|EventActorBeginOverlap
  (params (OtherActor :type Actor%20Object%20Reference))
  (if (Math|Boolean|ORBoolean (== (Utilities|GetClass OtherActor) "/Game/Grid/BP_block.BP_block_C") (== (Utilities|GetClass OtherActor) "/Game/Grid/BP_longblock.BP_longblock_C") (== (Utilities|GetClass OtherActor) "/Game/Grid/BP_longblock.BP_longblock_C"))
    (Variables|Default|SetIsTaken true)))

(event Collision|EventActorEndOverlap
  (params (OtherActor :type Actor%20Object%20Reference))
  (Variables|Default|SetIsTaken false))

(fn ConstructionScript)

(fn Initialize
  (bind _returnvalue (Components|GetOwner))
  (bind _plane (Variables|Default|GetPlane))
  (bind _boxextent (Collision|GetComponentBounds _plane))
  (bind (_x _y) (Math|Vector|BreakVector _boxextent))
  (Utilities|IsValid _returnvalue
    (:Is%20Valid
      (Transformation|AttachActorToActor _returnvalue "None" "SnapToTarget" "SnapToTarget" "KeepRelative" false)
      (Transformation|SetActorRelativeLocation (Math|Vector|MakeVector (* (* _x 2.0) (Variables|Default|GetColumn)) (* (* _y 2.0) (Variables|Default|GetRow)) 0.0)))))