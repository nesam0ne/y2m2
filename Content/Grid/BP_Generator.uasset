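; Grid puzzle manager that spawns a Rows by Columns board of BP_Tile actors and flags the WinIndex1 entries as winning tiles.
; BeginPlay builds the board, then positions and scales a clickable RefTie-material Plane to suit board size and win count.
; Clicking the Plane counts untaken winning tiles: all shows the next-level widget (dialogue on Level1_), some shows "more gems", none shows nothing.
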(event OnClicked(Plane)
  (params (TouchedComponent :type Primitive%20Component%20Object%20Reference) (ButtonPressed :type Key%20Structure :default "None"))
  (CallFunction|WinCheck))

(event Custom|WinCheck
  (Variables|Default|SetCount 0)
  (for _array_element (Variables|Default|GetWinIndex1)
    (if (not (Variables|/Game/Grid/BP_Tile.BP_Tile_C|GetIsTaken (Utilities|Array|Get(acopy) (Variables|Default|GetTiles) _array_element)))
      (Variables|Default|SetCount (+ (Variables|Default|GetCount) 1))))
  (if (== (Variables|Default|GetCount) (Utilities|Array|Length (Variables|Default|GetWinIndex1)))
    (bind _returnvalue (Game|GetCurrentLevelName true))
    (if (Utilities|Enum|Equal(Enum) _returnvalue "Level1_")
      (Viewport|RemoveAllWidgets)
      (bind _returnvalue_2 (UserInterface|CreateWidget "/Game/interface/W_dialogue_menu_3.W_dialogue_menu_3_C"))
      (UserInterface|Viewport|AddtoViewport _returnvalue_2 0)
      (else
        (bind _returnvalue_3 (UserInterface|CreateWidget "/Game/interface/W_nextTT.W_nextTT_C"))
        (UserInterface|Viewport|AddtoViewport _returnvalue_3 0)))
    (elif (> (Variables|Default|GetCount) 0)
      (bind _returnvalue_4 (UserInterface|CreateWidget "/Game/interface/W_moregems.W_moregems_C"))
      (UserInterface|Viewport|AddtoViewport _returnvalue_4 0))))

(event EventBeginPlay
  (CallFunction|InitializeTiles)
  (Variables|Default|SetCount 0)
  (if (== (Utilities|Array|Length (Variables|Default|GetTiles)) 4)
    (Transformation|SetRelativeTransform (Variables|Default|GetPlane) (Math|Transform|MakeTransform "360.000000,50.000000,60.000000" "0, 0, 0" "1.000000,1.000000,1.000000") false false)
    (elif (== (Utilities|Array|Length (Variables|Default|GetTiles)) 9)
      (Transformation|SetRelativeTransform (Variables|Default|GetPlane) (Math|Transform|MakeTransform "360.000000,100.000000,60.000000" "0, 0, 0" "1.000000,1.000000,1.000000") false false)
      (elif (and (== (Utilities|Array|Length (Variables|Default|GetTiles)) 16) (== (Utilities|Array|Length (Variables|Default|GetWinIndex1)) 1))
        (Transformation|SetRelativeTransform (Variables|Default|GetPlane) (Math|Transform|MakeTransform "500.000000,150.000000,60.000000" "0, 0, 0" "1.000000,1.000000,1.000000") false false)
        (elif (and (== (Utilities|Array|Length (Variables|Default|GetTiles)) 16) (== (Utilities|Array|Length (Variables|Default|GetWinIndex1)) 2))
          (Transformation|SetRelativeTransform (Variables|Default|GetPlane) (Math|Transform|MakeTransform "500.000000,145.000000,60.000000" "0, 0, 0" "1.000000,2.000000,1.000000") false false)
          (elif (and (== (Utilities|Array|Length (Variables|Default|GetTiles)) 16) (== (Utilities|Array|Length (Variables|Default|GetWinIndex1)) 3))
            (Transformation|SetRelativeTransform (Variables|Default|GetPlane) (Math|Transform|MakeTransform "500.000000,145.000000,60.000000" "0, 0, 0" "1.000000,3.000000,1.000000") false false)
            (elif (== (Utilities|Array|Length (Variables|Default|GetTiles)) 25)
              (Transformation|SetRelativeTransform (Variables|Default|GetPlane) (Math|Transform|MakeTransform "600.000000,200.000000,60.000000" "0, 0, 0" "1.000000,3.000000,1.000000") false false))))))))

(fn ConstructionScript
  (Rendering|Material|SetMaterial (Variables|Default|GetPlane) 0 (Variables|Default|GetRefTie)))

(fn InitializeTiles
  (CallFunction|ClearTiles)
  (for _index (range 0 (- (Variables|Default|GetRows) 1))
    (for _index_2 (range 0 (- (Variables|Default|GetColumns) 1))
      (bind _returnvalue (Game|SpawnActorfromClass "/Game/Grid/BP_Tile.BP_Tile_C" (Math|Transform|MakeTransform (Transformation|GetActorLocation) (Transformation|GetActorRotation)) "AlwaysSpawn" "MultiplyWithRoot" self _index _index_2 0))
      (Default|Initialize _returnvalue)
      (Utilities|Array|Add (Variables|Default|GetTiles) _returnvalue))
    (for _array_element (Variables|Default|GetWinIndex1)
      (Variables|/Game/Grid/BP_Tile.BP_Tile_C|SetIsWin (Utilities|Array|Get(acopy) (Variables|Default|GetTiles) _array_element) true)
      (Utilities|Array|SetArrayElem (Variables|Default|GetTiles) _array_element (Utilities|Array|Get(acopy) (Variables|Default|GetTiles) _array_element)))))

(fn ClearTiles
  (bind _tiles (Variables|Default|GetTiles))
  (if (> (Utilities|Array|Length (Variables|Default|GetTiles)) 0)
    (for _array_element _tiles
      (Actor|DestroyActor _array_element))
    (Utilities|Array|Clear _tiles)))